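; BP_LevelEnd is the level-end trigger that completes the level when the player character overlaps its sphere.
; The overlap disables player input and opens a Gate on Tick that VInterps the character toward the actor's root like a magnet, until Disablemagnet closes it.
; After a short delay, a DoOnce calls ThrowIngredients, passes LastLevel to the HUD and shows level completion through LevelComplete.
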(event OnComponentBeginOverlap(Sphere)
  (params (OverlappedComponent :type Primitive%20Component%20Object%20Reference) (OtherActor :type Actor%20Object%20Reference) (OtherComp :type Primitive%20Component%20Object%20Reference) (OtherBodyIndex :type Integer) (bFromSweep :type Boolean) (SweepResult :type Hit%20Result%20Structure%20%28by%20ref%29))
  (bind _asch_player_character (Utilities|Casting|CastToCH_PlayerCharacter OtherActor))
  (Input|DisableInput _asch_player_character (Game|GetPlayerController 0))
  (Utilities|FlowControl|Gate true) ; enters at Open
)

(event Custom|Disable%20magnet
  (Utilities|FlowControl|Gate true) ; enters at Close
)

(event EventBeginPlay)

(event Collision|EventActorBeginOverlap
  (params (OtherActor :type Actor%20Object%20Reference)))

(event EventTick
  (params (DeltaSeconds :type Float%20%28single-precision%29))
  (Variables|Default|SetDelta DeltaSeconds)
  (Utilities|FlowControl|Gate true
    (:Exit
      (Transformation|SetActorLocation (stale OnComponentBeginOverlap(Sphere) OtherActor) (Math|Interpolation|VInterpTo (Transformation|GetActorLocation (stale OnComponentBeginOverlap(Sphere) OtherActor)) (Transformation|GetWorldLocation (Variables|Default|GetDefaultSceneRoot)) (Variables|Default|GetDelta) 5.0) false false)
      (Utilities|FlowControl|Delay 0.5)
      (Utilities|FlowControl|DoOnce false
        (:Completed
          (Default|ThrowIngredients (stale OnComponentBeginOverlap(Sphere) _asch_player_character))
          (Variables|/Game/LD_UI/HUD.HUD_C|SetLast%20level? (Variables|/Game/LD_Blueprints/CH_PlayerCharacter.CH_PlayerCharacter_C|GetHUD%20reference (stale OnComponentBeginOverlap(Sphere) _asch_player_character)) (Variables|Default|GetLast%20Level?))
          (Default|LevelComplete (Variables|/Game/LD_Blueprints/CH_PlayerCharacter.CH_PlayerCharacter_C|GetHUD%20reference (stale OnComponentBeginOverlap(Sphere) _asch_player_character))))))))

(fn ConstructionScript)