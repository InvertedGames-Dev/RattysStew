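; BP_Collectable is an ingredient pickup (chilli, ham, carrot or eggplant) whose construction script sets mesh, transform and optional physics, and caches the first CH_PlayerCharacter.
; Tick adds looping BobCurve offsets to the mesh from a random start time, pins Mesh and Cube to a fixed world X plane, and keeps Cube unrotated.
; Collect runs once, reporting the type to the player, easing Cube toward the player's location, then destroying the actor.
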(event EventTick
  (params (DeltaSeconds :type Float%20%28single-precision%29))
  (bind _mesh (Variables|Default|GetMesh))
  (bind _cube (Variables|Default|GetCube))
  (bind _returnvalue (Transformation|GetWorldLocation _cube))
  (bind _returnvalue_2 (Transformation|GetWorldLocation _mesh))
  (bind (_x _y _z) (Math|Vector|BreakVector _returnvalue_2))
  (if (== (Math|Float|Clamp(Float) (+ (Variables|Default|GetCurve%20Time) 0.01) 0.0 2.0) 2.0)
    (Variables|Default|SetCurve%20Time 0.0)
    (else
      (Variables|Default|SetCurve%20Time (Math|Float|Clamp(Float) (+ (Variables|Default|GetCurve%20Time) 0.01) 0.0 2.0))))
  (Transformation|SetWorldLocation _mesh (+ _returnvalue_2 (Math|Vector|MakeVector 0.0 0.0 (.z (Math|Curves|GetVectorValue (Variables|Default|GetBobCurve) (Variables|Default|GetCurve%20Time))))) false false)
  (Transformation|SetWorldLocation _mesh (Math|Vector|MakeVector 1.2e+03 _y _z) false false)
  (Transformation|SetWorldLocation _cube (Math|Vector|MakeVector 1.2e+03 (.y _returnvalue) (.z _returnvalue)) false false)
  (Transformation|SetWorldRotation _cube "0, 0, 0" false false))

(event EventCollect
  (Utilities|FlowControl|DoOnce false
    (:Completed
      (Default|CollectedIngredient (Variables|Default|GetPlayer%20Character) (Variables|Default|GetCollectableType))
      (Components|MoveComponentTo (Variables|Default|GetCube) (Transformation|GetWorldLocation (Variables|/Script/Engine.Actor|GetRootComponent (Variables|Default|GetPlayer%20Character))) "0, 0, 0" true true 0.1 false)
      (Actor|DestroyActor))))

(event EventBeginPlay
  (Variables|Default|SetCurve%20Time (Math|Random|RandomFloatinRange 0.0 2.0)))

(fn ConstructionScript
  (bind _collectabletype (Variables|Default|GetCollectableType))
  (bind _mesh (Variables|Default|GetMesh))
  (bind _outactors (Actor|GetAllActorsOfClass "/Game/LD_Blueprints/CH_PlayerCharacter.CH_PlayerCharacter_C"))
  (Variables|Default|SetPlayer%20Character (Utilities|Array|Get(acopy) _outactors))
  (Physics|SetSimulatePhysics (Variables|Default|GetCube) (Variables|Default|GetSimulate%20Physics?))
  (Components|StaticMesh|SetStaticMesh (Variables|Default|GetMesh) (Utilities|Select :Index _collectabletype :NewEnumerator0 "/Game/LD_Geometry/SmallProps/Chilli.Chilli" :NewEnumerator1 "/Game/LD_Geometry/SmallProps/Ham.Ham" :NewEnumerator2 "/Game/LD_Geometry/SmallProps/Carrot.Carrot" :NewEnumerator3 "/Game/LD_Geometry/SmallProps/eggplant.eggplant"))
  (switch Utilities|FlowControl|Switch|SwitchonE_CollectableType _collectabletype
    (:NewEnumerator0
      (Transformation|SetRelativeRotation _mesh "0.000000,0.000000,0.000000" false false)
      (Transformation|SetRelativeScale3D _mesh "1.000000,1.000000,1.000000"))
    (:NewEnumerator1
      (Transformation|SetRelativeRotation _mesh "20.000000,40.000000,60.000000" false false)
      (Transformation|SetRelativeScale3D _mesh "0.250000,0.250000,0.250000"))
    (:NewEnumerator2
      (Transformation|SetRelativeRotation _mesh "29.498697,-5.725128,88.491684" false false)
      (Transformation|SetRelativeScale3D _mesh "0.500000,0.500000,0.500000"))
    (:NewEnumerator3
      (Transformation|SetRelativeRotation _mesh "-9.846558,79.848969,1.753768" false false)
      (Transformation|SetRelativeScale3D _mesh "0.200000,0.200000,0.200000"))))