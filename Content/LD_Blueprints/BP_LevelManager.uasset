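; BP_LevelManager snapshots the level's enemies, spice containers and spice pickups so the level can be reset to that state.
; CollectAllEntities runs on construction and BeginPlay, storing each actor's class and transform, plus two points for enemies, in three arrays.
; ResetLevel destroys every current actor of those three types, respawns them from the stored arrays and prints a confirmation.
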(event Custom|Reset%20Level
  (bind _outactors (Actor|GetAllActorsOfClass "/Game/LD_Blueprints/BP_BaseEnemy.BP_BaseEnemy_C"))
  (for _array_element _outactors
    (Actor|DestroyActor _array_element))
  (for _array_element_2 (Variables|Default|GetEnemies)
    (Game|SpawnActorfromClass (.EnemyClass (Utilities|Struct|BreakS_Enemies _array_element_2)) (.Transform (Utilities|Struct|BreakS_Enemies _array_element_2)) "Undefined" 0 (.Point1 (Utilities|Struct|BreakS_Enemies _array_element_2)) (.Point2 (Utilities|Struct|BreakS_Enemies _array_element_2)) 0))
  (bind _outactors_2 (Actor|GetAllActorsOfClass "/Game/LD_Blueprints/BP_SpiceContainer.BP_SpiceContainer_C"))
  (for _array_element_3 _outactors_2
    (Actor|DestroyActor _array_element_3))
  (for _array_element_4 (Variables|Default|GetSpice%20Containers)
    (Game|SpawnActorfromClass (.SpiceContainer (Utilities|Struct|BreakS_SpiceContainers _array_element_4)) (.Transform (Utilities|Struct|BreakS_SpiceContainers _array_element_4)) "Undefined" 0 false 0))
  (bind _outactors_3 (Actor|GetAllActorsOfClass "/Game/LD_Blueprints/BP_Spice.BP_Spice_C"))
  (for _array_element_5 _outactors_3
    (Actor|DestroyActor _array_element_5))
  (for _array_element_6 (Variables|Default|GetSpice)
    (Game|SpawnActorfromClass (.Spice (Utilities|Struct|BreakS_Spices _array_element_6)) (.Transform (Utilities|Struct|BreakS_Spices _array_element_6)) "Undefined" 0 false 0))
  (Development|PrintString "Level Reset"))

(event EventBeginPlay
  (CallFunction|CollectAllEntities))

(fn ConstructionScript
  (CallFunction|CollectAllEntities))

(fn CollectAllEntities
  (Utilities|Array|Clear (Variables|Default|GetEnemies))
  (Utilities|Array|Clear (Variables|Default|GetSpice%20Containers))
  (Utilities|Array|Clear (Variables|Default|GetSpice))
  (bind _outactors (Actor|GetAllActorsOfClass "/Game/LD_Blueprints/BP_BaseEnemy.BP_BaseEnemy_C"))
  (for _array_element _outactors
    (Utilities|Array|Add (Variables|Default|GetEnemies) (Utilities|Struct|MakeS_Enemies (Variables|/Game/LD_Blueprints/BP_BaseEnemy.BP_BaseEnemy_C|GetEnemy%20Class _array_element) (Transformation|GetActorTransform _array_element) (Variables|/Game/LD_Blueprints/BP_BaseEnemy.BP_BaseEnemy_C|GetPoint%201 _array_element) (Variables|/Game/LD_Blueprints/BP_BaseEnemy.BP_BaseEnemy_C|GetPoint%202 _array_element))))
  (bind _outactors_2 (Actor|GetAllActorsOfClass "/Game/LD_Blueprints/BP_SpiceContainer.BP_SpiceContainer_C"))
  (for _array_element_2 _outactors_2
    (Utilities|Array|Add (Variables|Default|GetSpice%20Containers) (Utilities|Struct|MakeS_SpiceContainers (Utilities|GetClass _array_element_2) (Transformation|GetActorTransform _array_element_2))))
  (bind _outactors_3 (Actor|GetAllActorsOfClass "/Game/LD_Blueprints/BP_Spice.BP_Spice_C"))
  (for _array_element_3 _outactors_3
    (Utilities|Array|Add (Variables|Default|GetSpice) (Utilities|Struct|MakeS_Spices (Utilities|GetClass _array_element_3) (Transformation|GetActorTransform _array_element_3)))))