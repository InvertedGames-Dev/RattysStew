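; BP_1UP is an extra-life style coffee bean pickup that increments the player's UPs value when collected.
; Tick bobs the bean along a looping curve from a random start time, pins bean and cube to a fixed X plane and zeroes cube rotation.
; Collect plays a sound, then once only adds the 1UP, eases the cube toward the player and destroys the actor.
; The construction script caches the player and sets optional cube physics.
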(event EventTick
  (params (DeltaSeconds :type Float%20%28single-precision%29))
  (bind _coffeebean (Variables|Default|GetCoffeeBean))
  (bind _cube (Variables|Default|GetCube))
  (bind _returnvalue (Transformation|GetWorldLocation _cube))
  (bind _returnvalue_2 (Transformation|GetWorldLocation _coffeebean))
  (bind (_x _y _z) (Math|Vector|BreakVector _returnvalue_2))
  (if (== (Math|Float|Clamp(Float) (+ (Variables|Default|GetCurve%20Time) 0.01) 0.0 2.0) 2.0)
    (Variables|Default|SetCurve%20Time 0.0)
    (else
      (Variables|Default|SetCurve%20Time (Math|Float|Clamp(Float) (+ (Variables|Default|GetCurve%20Time) 0.01) 0.0 2.0))))
  (Transformation|SetWorldLocation _coffeebean (+ _returnvalue_2 (Math|Vector|MakeVector 0.0 0.0 (.z (Math|Curves|GetVectorValue (Variables|Default|GetBobCurve) (Variables|Default|GetCurve%20Time))))) false false)
  (Transformation|SetWorldLocation _coffeebean (Math|Vector|MakeVector 1.2e+03 _y _z) false false)
  (Transformation|SetWorldLocation _cube (Math|Vector|MakeVector 1.2e+03 (.y _returnvalue) (.z _returnvalue)) false false)
  (Transformation|SetWorldRotation _cube "0, 0, 0" false false))

(event EventCollect
  (bind _player_character (Variables|Default|GetPlayer%20Character))
  (Audio|SpawnSoundatLocation "/Game/LD_Sound/SFX/Collected.Collected" (Transformation|GetActorLocation self))
  (Utilities|FlowControl|DoOnce false
    (:Completed
      (Variables|/Game/LD_Blueprints/CH_PlayerCharacter.CH_PlayerCharacter_C|SetUPs _player_character (Utilities|Enum|ByteToEnumE_1UP (+ (Variables|/Game/LD_Blueprints/CH_PlayerCharacter.CH_PlayerCharacter_C|GetUPs _player_character) 1)))
      (Components|MoveComponentTo (Variables|Default|GetCube) (Transformation|GetWorldLocation (Variables|/Script/Engine.Actor|GetRootComponent (Variables|Default|GetPlayer%20Character))) "0, 0, 0" true true 0.1 false)
      (Actor|DestroyActor))))

(event EventBeginPlay
  (Variables|Default|SetCurve%20Time (Math|Random|RandomFloatinRange 0.0 2.0)))

(fn ConstructionScript
  (bind _outactors (Actor|GetAllActorsOfClass "/Game/LD_Blueprints/CH_PlayerCharacter.CH_PlayerCharacter_C"))
  (Variables|Default|SetPlayer%20Character (Utilities|Array|Get(acopy) _outactors))
  (Physics|SetSimulatePhysics (Variables|Default|GetCube) (Variables|Default|GetSimulate%20Physics?)))