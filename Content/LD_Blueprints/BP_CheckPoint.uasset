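; BP_CheckPoint is a checkpoint actor, shown as an umbrella that stands open while it is the player's active checkpoint.
; Any overlap with its sphere sends NewCheckpointMessage with itself to the overlapping actor and plays a checkpoint sound.
; Tick swaps the open or closed mesh by comparing itself to the player's CheckPoint.
; The construction script caches the first CH_PlayerCharacter found in the level.
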(event OnComponentBeginOverlap(Sphere)
  (params (OverlappedComponent :type Primitive%20Component%20Object%20Reference) (OtherActor :type Actor%20Object%20Reference) (OtherComp :type Primitive%20Component%20Object%20Reference) (OtherBodyIndex :type Integer) (bFromSweep :type Boolean) (SweepResult :type Hit%20Result%20Structure%20%28by%20ref%29))
  (Class|BPIInteract|NewCheckpoint(Message) OtherActor self)
  (Audio|PlaySound2D "/Game/LD_Sound/SFX/SFX_Checkpoint_Cue.SFX_Checkpoint_Cue"))

(event EventBeginPlay)

(event Collision|EventActorBeginOverlap
  (params (OtherActor :type Actor%20Object%20Reference)))

(event EventTick
  (params (DeltaSeconds :type Float%20%28single-precision%29))
  (Components|StaticMesh|SetStaticMesh (Variables|Default|GetStaticMesh) (select (== (Variables|/Game/LD_Blueprints/CH_PlayerCharacter.CH_PlayerCharacter_C|GetCheckPoint (Variables|Default|GetPlayer%20Character)) self) "/Game/LD_Geometry/SmallProps/umbrella_opened.umbrella_opened" "/Game/LD_Geometry/SmallProps/Umbrella_Closed.Umbrella_Closed")))

(fn ConstructionScript
  (bind _outactors (Actor|GetAllActorsOfClass "/Game/LD_Blueprints/CH_PlayerCharacter.CH_PlayerCharacter_C"))
  (Variables|Default|SetPlayer%20Character (Utilities|Array|Get(acopy) _outactors)))