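; BP_Spice is a collectible spice pickup that bobs in place and adds to the player's spice count.
; Each Tick advances a looping curve time by a fixed, frame-rate-dependent step and adds the bob curve's Z value to the sphere's world location.
; Collect increments Spice on the player character, cached in the construction script via GetAllActorsOfClass, then destroys the pickup.
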(event EventTick
  (params (DeltaSeconds :type Float%20%28single-precision%29))
  (bind _sphere (Variables|Default|GetSphere))
  (if (== (Math|Float|Clamp(Float) (+ (Variables|Default|GetCurve%20Time) 0.01) 0.0 2.0) 2.0)
    (Variables|Default|SetCurve%20Time 0.0)
    (else
      (Variables|Default|SetCurve%20Time (Math|Float|Clamp(Float) (+ (Variables|Default|GetCurve%20Time) 0.01) 0.0 2.0))))
  (Transformation|SetWorldLocation _sphere (+ (Transformation|GetWorldLocation _sphere) (Math|Vector|MakeVector 0.0 0.0 (.z (Math|Curves|GetVectorValue (Variables|Default|GetBobCurve) (Variables|Default|GetCurve%20Time))))) false false))

(event EventCollect
  (bind _player_character (Variables|Default|GetPlayer%20Character))
  (bind _result (Math|Integer|IncrementInt (Variables|/Game/LD_Blueprints/CH_PlayerCharacter.CH_PlayerCharacter_C|GetSpice _player_character))
    (:%20%20
      (Variables|/Game/LD_Blueprints/CH_PlayerCharacter.CH_PlayerCharacter_C|SetSpice _player_character _result)
      (Actor|DestroyActor))))

(fn ConstructionScript
  (bind _outactors (Actor|GetAllActorsOfClass "/Game/LD_Blueprints/CH_PlayerCharacter.CH_PlayerCharacter_C"))
  (Variables|Default|SetPlayer%20Character (Utilities|Array|Get(acopy) _outactors)))