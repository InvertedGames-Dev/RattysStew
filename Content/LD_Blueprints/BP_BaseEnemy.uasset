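; BP_BaseEnemy is a base enemy actor that damages the player on contact and is destroyed when attacked.
; Sphere overlap calls Damage on a non-immune CH_PlayerCharacter, passing the sphere's world location.
; The Attack event destroys the enemy, first bouncing the player if the attack came from the air.
; The Construction Script caches the first player character found in the level and the enemy's own class.
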(event OnComponentBeginOverlap(Sphere)
  (params (OverlappedComponent :type Primitive%20Component%20Object%20Reference) (OtherActor :type Actor%20Object%20Reference) (OtherComp :type Primitive%20Component%20Object%20Reference) (OtherBodyIndex :type Integer) (bFromSweep :type Boolean) (SweepResult :type Hit%20Result%20Structure%20%28by%20ref%29))
  (bind _asch_player_character (Utilities|Casting|CastToCH_PlayerCharacter OtherActor))
  (if (not (Variables|/Game/LD_Blueprints/CH_PlayerCharacter.CH_PlayerCharacter_C|GetImmune _asch_player_character))
    (Default|Damage _asch_player_character (Transformation|GetWorldLocation (Variables|Default|GetSphere)))))

(event EventAttack
  (params (Attack%20From%20Air? :type Boolean))
  (if Attack%20From%20Air?
    (Default|Bounce (Variables|Default|GetPlayerCharacter) 1e+03))
  (Actor|DestroyActor))

(fn ConstructionScript
  (bind _outactors (Actor|GetAllActorsOfClass "/Game/LD_Blueprints/CH_PlayerCharacter.CH_PlayerCharacter_C"))
  (Variables|Default|SetPlayerCharacter (Utilities|Array|Get(acopy) _outactors))
  (Variables|Default|SetEnemy%20Class (Utilities|GetClass self)))