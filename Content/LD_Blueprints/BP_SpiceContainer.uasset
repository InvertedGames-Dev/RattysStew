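; BP_SpiceContainer is a breakable container that bursts into spice pickups when attacked.
; Its Attack event bounces the player if the hit comes from the air, spawns a random number of small BP_Spice actors around SpiceSpawner, then destroys the container.
; A variable sets whether spawned spice simulates physics.
; The construction script caches the first CH_PlayerCharacter found in the level.
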(event EventAttack
  (params (Attack%20From%20Air? :type Boolean))
  (if Attack%20From%20Air?
    (Default|Bounce (Variables|Default|GetPlayer%20Character) 1e+03))
  (for _index (range 0 (Math|Random|RandomIntegerinRange 10 20))
    (Game|SpawnActorfromClass "/Game/LD_Blueprints/BP_Spice.BP_Spice_C" (Math|Transform|MakeTransform (+ (Transformation|GetWorldLocation (Variables|Default|GetSpiceSpawner)) (Math|Vector|MakeVector 0.0 (Math|Random|RandomFloatinRange -1e+02 1e+02) (Math|Random|RandomFloatinRange -1e+02 1e+02))) "0, 0, 0" "0.200000,0.200000,0.200000") "Undefined" 0 (Variables|Default|GetSpawned%20spice%20will%20simulate%20physics) 0))
  (Actor|DestroyActor))

(fn ConstructionScript
  (bind _outactors (Actor|GetAllActorsOfClass "/Game/LD_Blueprints/CH_PlayerCharacter.CH_PlayerCharacter_C"))
  (Variables|Default|SetPlayer%20Character (Utilities|Array|Get(acopy) _outactors)))